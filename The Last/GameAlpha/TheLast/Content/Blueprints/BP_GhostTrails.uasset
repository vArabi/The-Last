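; Afterimage actor that shows a frozen copy of the player character's pose as a fading ghost trail, then removes itself.
; On BeginPlay it copies the player mesh's pose onto the Fantasminha poseable mesh and gives each material slot a dynamic instance of MI_GhostTrails.
; The Opacity timeline drives the Opacity parameter on those instances and destroys the actor when it finishes.
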(event `self.ReceiveBeginPlay`
  (bind _asthird_person_character (cast `/Game/ThirdPersonBP/Blueprints/ThirdPersonCharacter` (`GameplayStatics.GetPlayerPawn` 0)))
  (set `self.PlayerCharacterRef` _asthird_person_character)
  (`self.GhostTrails`))

(event `GhostTrails`
  (for _ (`MeshComponent.GetMaterials` (`self.Fantasminha`))
    (bind _returnvalue (`KismetMaterialLibrary.CreateDynamicMaterialInstance` "/Game/Materials/MI_GhostTrails.MI_GhostTrails"))
    (bind _returnvalue_2 (`KismetArrayLibrary.Array_Add` (`self.DynamicMats`) _returnvalue))
    (`PrimitiveComponent.SetMaterial` (`self.Fantasminha`) _returnvalue_2 _returnvalue)
    (`PoseableMeshComponent.CopyPoseFromSkeletalComponent` (`self.Fantasminha`) (`Character.Mesh` (`self.PlayerCharacterRef`)))
    (`TimelineComponent.PlayFromStart` (`self.Opacity`))))

(fn `UserConstructionScript`)