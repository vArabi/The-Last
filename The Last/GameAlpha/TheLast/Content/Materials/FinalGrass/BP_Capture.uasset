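; Scene capture actor that follows player 0 to record components tagged GrassTrail, apparently for grass trail materials.
; CustomEvent writes the capture's ortho width to MPC_Capture, limits SceneCapture to tagged components on tagged actors, and starts a fast looping timer.
; Each MoveTarget tick matches the player's XY at fixed height and publishes CaptureLocation to the collection.
; MoveCapture and SetCaptureSize duplicate this logic without a collection set and are not called here.
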(event `CustomEvent`
  (`KismetMaterialLibrary.SetScalarParameterValue` "/Game/Materials/FinalGrass/MPC_Capture.MPC_Capture" "CaptureSize" (`SceneCaptureComponent2D.OrthoWidth` (`self.SceneCapture`)))
  (`KismetSystemLibrary.K2_SetTimer` null "MoveTarget" 0.01 true)
  (bind _outactors (`GameplayStatics.GetAllActorsWithTag` "GrassTrail"))
  (for _array_element _outactors
    (for _array_element_2 (`self.GetComponentsByTag` _array_element "/Script/Engine.PrimitiveComponent" "GrassTrail")
      (`SceneCaptureComponent.ShowOnlyComponent` (`self.SceneCapture`) _array_element_2))))

(event `MoveTarget`
  (bind (_returnvalue_x _returnvalue_y _returnvalue_z) (`KismetMathLibrary.BreakVector` (`self.K2_GetActorLocation`)))
  (bind (_returnvalue_x_2 _returnvalue_y_2) (`KismetMathLibrary.BreakVector` (`self.K2_GetActorLocation` (`GameplayStatics.GetPlayerCharacter` 0))))
  (`self.K2_SetActorLocation` (`KismetMathLibrary.MakeVector` _returnvalue_x_2 _returnvalue_y_2 _returnvalue_z))
  (`KismetMaterialLibrary.SetVectorParameterValue` "/Game/Materials/FinalGrass/MPC_Capture.MPC_Capture" "CaptureLocation" (`KismetMathLibrary.Conv_VectorToLinearColor` (`self.K2_GetActorLocation`))))

(fn `MoveCapture`
  (bind (_returnvalue_x _returnvalue_y _returnvalue_z) (`KismetMathLibrary.BreakVector` (`self.K2_GetActorLocation`)))
  (bind (_returnvalue_x_2 _returnvalue_y_2) (`KismetMathLibrary.BreakVector` (`self.K2_GetActorLocation` (`GameplayStatics.GetPlayerCharacter` 0))))
  (`self.K2_SetActorLocation` (`KismetMathLibrary.MakeVector` _returnvalue_x_2 _returnvalue_y_2 _returnvalue_z))
  (`KismetMaterialLibrary.SetVectorParameterValue` null "CaptureLocation" (`KismetMathLibrary.Conv_VectorToLinearColor` (`self.K2_GetActorLocation`))))

(fn `SetCaptureSize`
  (`KismetMaterialLibrary.SetScalarParameterValue` null "CaptureSize" (`SceneCaptureComponent2D.OrthoWidth` (`self.SceneCapture`))))

(fn `UserConstructionScript`)